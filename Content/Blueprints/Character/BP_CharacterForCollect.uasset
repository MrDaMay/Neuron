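; Player character Blueprint that collects items and starts with a rifle through InitWeapon on BeginPlay.
; Capsule overlaps send enter and leave interface messages to the other actor, intended for item-side widget display, and store or clear a single InteractableActor.
; Pressing E sends CollectItem to that actor if valid.
; Tick prints the current weapon's fire timer and rate of fire for debugging.
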(event `self.ReceiveBeginPlay`
  (`self.InitWeapon` "Rifle" (make `AdditionalWeaponInfo` 100)))

(event `self.ReceiveActorBeginOverlap`
  (params (OtherActor :type "Actor Object Reference")))

(event `self.ReceiveTick`
  (params (DeltaSeconds :type "Float (single-precision)"))
  (bind _currentweapon (`self.CurrentWeapon`))
  (`KismetSystemLibrary.PrintString` (`KismetStringLibrary.Conv_DoubleToString` (`NR_Weapon.FireTimer` _currentweapon)) true true (struct :`G` 0.66 :`B` 1.0 :`A` 1.0) 0.0)
  (`KismetSystemLibrary.PrintString` (`KismetStringLibrary.Conv_DoubleToString` (`NR_Weapon.WeaponRateOfFire` _currentweapon)) true true (struct :`R` 0.009697 :`G` 1.0 :`A` 1.0) 0.0))

(event `self.CapsuleComponent.OnComponentBeginOverlap`
  (params (OverlappedComponent :type "PrimitiveComponent Object Reference") (OtherActor :type "Actor Object Reference") (OtherComp :type "PrimitiveComponent Object Reference") (OtherBodyIndex :type Integer) (bFromSweep :type Boolean) (SweepResult :type "HitResult Structure (by ref)"))
  ;[1 1 1] Для появления и скрытия виджета. Логику добавим в сами подбираемые предметы
  (message `NR_CollectableInterface.EnteredInteractionZone` OtherActor self)
  (set `self.InteractableActor` OtherActor))

(event `self.CapsuleComponent.OnComponentEndOverlap`
  (params (OverlappedComponent :type "PrimitiveComponent Object Reference") (OtherActor :type "Actor Object Reference") (OtherComp :type "PrimitiveComponent Object Reference") (OtherBodyIndex :type Integer))
  ;[1 1 1] Для появления и скрытия виджета. Логику добавим в сами подбираемые предметы
  (message `NR_CollectableInterface.LeftInteractionZone` OtherActor self)
  (set `self.InteractableActor` null))

(event `Key|E`
  (params (Key :type "Key Structure"))
  (bind _interactableactor (`self.InteractableActor`))
  (:`Pressed`
    (`/Engine/EditorBlueprintResources/StandardMacros.IsValid` _interactableactor
      (:`Is Valid`
        (message `NR_CollectableInterface.CollectItem` _interactableactor self)))))

(fn `UserConstructionScript`)