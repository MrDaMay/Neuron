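; BP_BootHelper is a tutorial helper actor that highlights its skeletal mesh and shows an E prompt.
; On BeginPlay it binds to the BP_PC_Tutorial controller's PushE and Eoff events.
; PushE turns the mesh yellow, shows the widget and starts a FlipFlop/Delay loop blinking E every half second.
; Eoff restores the material and hides the widget but leaves that loop running.
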(event `CustomEvent_0`
  (`PrimitiveComponent.SetMaterial` (`self.SkeletalMesh`) 0 "/Game/Envinronment/RobotHelper/Textures/M_BootHelper.M_BootHelper")
  (`SceneComponent.SetVisibility` (`self.Widget`) false false))

(event `self.ReceiveBeginPlay`
  (bind _as_bp_pc_tutorial (`self.As BP PC Tutorial`))
  (bind _asbp_pc_tutorial (cast `/Game/Blueprints/Tutorial/BP_PC_Tutorial` (`GameplayStatics.GetPlayerController` 0)))
  (set `self.As BP PC Tutorial` _asbp_pc_tutorial)
  (`PrimitiveComponent.SetMaterial` (`self.SkeletalMesh`) 0 "/Game/Envinronment/RobotHelper/Textures/M_BootHelper.M_BootHelper")
  (`SceneComponent.SetVisibility` (`self.Widget`) false false)
  (`|ExecutionSequence`
    (:`then_0`
      (add `/Game/Blueprints/Tutorial/BP_PC_Tutorial.PushE` _as_bp_pc_tutorial (delegate `CustomEvent`)))
    (:`then_1`
      (add `/Game/Blueprints/Tutorial/BP_PC_Tutorial.Eoff` _as_bp_pc_tutorial (delegate `CustomEvent_0`)))))

(event `CustomEvent`
  (bind _e (`self.e`))
  (`PrimitiveComponent.SetMaterial` (`self.SkeletalMesh`) 0 "/Game/Envinronment/RobotHelper/Textures/M_BootHelperYellow.M_BootHelperYellow")
  (`SceneComponent.SetVisibility` (`self.Widget`) true false)
  (`/Engine/EditorBlueprintResources/StandardMacros.FlipFlop` :!label _label
    (:`A`
      (`SceneComponent.SetVisibility` _e true false)
      (`KismetSystemLibrary.Delay` 0.5)
      (goto _label))
    (:`B`
      (`SceneComponent.SetVisibility` _e false false)
      (`KismetSystemLibrary.Delay` 0.5)
      (goto _label))))

(fn `UserConstructionScript`)