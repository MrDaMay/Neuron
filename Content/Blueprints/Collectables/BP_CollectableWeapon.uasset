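; BP_CollectableWeapon is a collectable weapon actor that a character can pick up in the world.
; On collection it calls InitWeapon on a valid character with its WeaponName, then destroys itself.
; Entering and leaving the interaction zone both call OpenPickupWidgetEvent on the character's BP_PlayerController with the weapon name; no separate close call is made.
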(event `NR_CollectableInterface.CollectItem`
  (params (Character :type "NR_Character Object Reference"))
  (`/Engine/EditorBlueprintResources/StandardMacros.IsValid` Character
    (:`Is Valid`
      (`NR_Character.InitWeapon` Character (`self.WeaponName`))
      (`self.K2_DestroyActor`))))

(event `NR_CollectableInterface.LeftInteractionZone`
  (params (Character :type "NR_Character Object Reference"))
  (bind _asbp_player_controller (cast `/Game/Blueprints/Game/BP_PlayerController` (`Pawn.GetController` Character)))
  (`/Game/Blueprints/Game/BP_PlayerController.OpenPickupWidget_Event` _asbp_player_controller (`self.WeaponName`)))

(event `NR_CollectableInterface.EnteredInteractionZone`
  (params (Character :type "NR_Character Object Reference"))
  (bind _asbp_player_controller (cast `/Game/Blueprints/Game/BP_PlayerController` (`Pawn.GetController` Character)))
  (`/Game/Blueprints/Game/BP_PlayerController.OpenPickupWidget_Event` _asbp_player_controller (`self.WeaponName`)))

(fn `UserConstructionScript`
  (`parent.UserConstructionScript`))