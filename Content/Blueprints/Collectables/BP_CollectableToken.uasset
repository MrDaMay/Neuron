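; Collectable token Blueprint meant to be picked up when a character enters its interaction zone.
; The EnteredInteractionZone event forwards the character to CollectItem, which checks that the character's TokenComponent is valid.
; Nothing follows that check, so the graph awards no token, and the construction script only calls its parent.
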(event `NR_CollectableInterface.EnteredInteractionZone`
  (params (Character :type "NR_Character Object Reference"))
  (`NR_CollectableInterface.CollectItem` Character))

(event `NR_CollectableInterface.CollectItem`
  (params (Character :type "NR_Character Object Reference"))
  (`/Engine/EditorBlueprintResources/StandardMacros.IsValid` (`NR_Character.TokenComponent` Character)))

(fn `UserConstructionScript`
  (`parent.UserConstructionScript`))