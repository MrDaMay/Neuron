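; BP_EnemyBoss is the boss enemy Blueprint, exposing its attack action and combat state checks.
; The Attack event calls StartAttackEnemy, while CanAttack and CanMove return the results of CanEnemyAttack and CanEnemyMove.
; IsAlive reads its result from the HealthComponent.
; The graphs are thin wrappers with no logic of their own, and the default events and construction script are empty.
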(event `/Game/Blueprints/Enemy/AI/Base/BPI_CombatEnemy.Attack`
  (`self.StartAttackEnemy`))

(fn `CanAttack`
  (returns (IsCanAttack :type Boolean))
  (bind _returnvalue (`self.CanEnemyAttack`))
  (return _returnvalue))

(fn `CanMove`
  (returns (IsCanMove :type Boolean))
  (bind _returnvalue (`self.CanEnemyMove`))
  (return _returnvalue))

(fn `IsAlive`
  (returns (IsAlive :type Boolean))
  (bind _returnvalue (`NR_HealthComponent.GetIsAlive` (`self.HealthComponent`)))
  (return _returnvalue))

(fn `UserConstructionScript`)