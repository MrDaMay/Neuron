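; Shooter enemy Blueprint that exposes attack, movement and life-state hooks as thin wrappers.
; The Attack event calls StartAttackEnemy, while CanAttack and CanMove return CanEnemyAttack and CanEnemyMove.
; IsAlive reads its result from the HealthComponent.
; The shooting logic itself lives outside these graphs, and BeginPlay, overlap and Tick are disabled stubs.
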(event `/Game/Blueprints/Enemy/AI/Base/BPI_CombatEnemy.Attack`
  (`self.StartAttackEnemy`))

(fn `CanAttack`
  (returns (IsCanAttack :type Boolean))
  (bind _returnvalue (`self.CanEnemyAttack`))
  (return _returnvalue))

(fn `CanMove`
  (returns (IsCanMove :type Boolean))
  (bind _returnvalue (`self.CanEnemyMove`))
  (return _returnvalue))

(fn `IsAlive`
  (returns (IsAlive :type Boolean))
  (bind _returnvalue (`NR_HealthComponent.GetIsAlive` (`self.HealthComponent`)))
  (return _returnvalue))

(fn `UserConstructionScript`
  (`parent.UserConstructionScript`))