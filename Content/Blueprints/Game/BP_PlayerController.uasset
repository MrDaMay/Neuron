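; Player controller that sets up the in-game HUD, level music and keys for opening UI screens.
; Game state events switch music to the boss track when waves end and allow the token widget toggle until the boss phase starts.
; Bound events drive the token widget and a pausing end-game menu, which also has a debug key.
; Other keys spawn dialog and leaderboard widgets.
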(event Custom|OnAchieveOpen
  (bind _self self)
  (bind _returnvalue (UserInterface|CreateWidget "/Game/Blueprints/Widgets/BPW_EndGameMenu.BPW_EndGameMenu_C"))
  (UserInterface|Viewport|AddtoViewport _returnvalue 0)
  (Game|SetGamePaused true)
  (Input|SetInputModeUIOnly _self _returnvalue "DoNotLock" false)
  (Variables|Default|SetbShowMouseCursor _self true))

(event Custom|OnTokenWidget
  (Default|OpenCloseTokenWidget (Variables|Default|GetUserInterface)))

(event Custom|OnWavePhaseEnds_Event
  (Audio|Components|Audio|SetSound (Variables|Default|GetMusic) "/Game/Fx_Effects/Sound/Music/OST_BossFigth.OST_BossFigth")
  (Variables|Default|SetbIsAvailable true)
  (Development|PrintString "Wave Ended!"))

(event Custom|OnBossPhaseStarts_Event
  (params (Boss :type NR%20Enemy%20Boss%20Class%20Reference))
  (Variables|Default|SetbIsAvailable false))

(event EventBeginPlay
  (bind _returnvalue (UserInterface|CreateWidget "/Game/Blueprints/Widgets/BPW_InGame.BPW_InGame_C"))
  (UserInterface|Viewport|AddtoViewport _returnvalue 0)
  (bind _output_get (Variables|Default|SetUserInterface _returnvalue))
  (Input|SetInputModeGameandUI self _output_get "DoNotLock" true false)
  (bind _returnvalue_2 (Audio|CreateSound2D (Utilities|Select :Index (Math|Random|RandomIntegerinRange 0 1) :Option%200 "/Game/Fx_Effects/Sound/Music/Level_OST_vol1.Level_OST_vol1" :Option%201 "/Game/Fx_Effects/Sound/Music/Level_OST_vol2.Level_OST_vol2") 1.0 1.0 0.0 0))
  (Variables|Default|SetMusic _returnvalue_2)
  (EventDispatchers|BindEventtoOnOpenTokenWidget (delegate Custom|OnTokenWidget))
  (EventDispatchers|BindEventtoOnOpenAchieveWidget (delegate Custom|OnAchieveOpen))
  (bind _asnr_game_state (Utilities|Casting|CastToNR_GameState (Game|GetGameState)))
  (EventDispatchers|AssignOnWavePhaseEnds _asnr_game_state (delegate Custom|OnWavePhaseEnds_Event))
  (EventDispatchers|AssignOnBossPhaseStarts _asnr_game_state (delegate Custom|OnBossPhaseStarts_Event)))

(event EventTick
  (params (DeltaSeconds :type Float%20%28single-precision%29)))

(event Input|KeyboardEvents|DebugKeyG
  (params (Key :type Key%20Structure :default "None") (ActionValue :type Input%20Action%20Value%20Structure))
  (:Pressed
    (CallFunction|OnAchieveOpen)))

(event Input|KeyboardEvents|T
  (params (Key :type Key%20Structure :default "None"))
  (:Pressed
    (if (Variables|Default|GetbIsAvailable)
      (CallFunction|OnTokenWidget))))

(event Input|KeyboardEvents|R
  (params (Key :type Key%20Structure :default "None"))
  (:Pressed
    (bind _returnvalue (UserInterface|CreateWidget "/Game/Blueprints/Widgets/BPW_DialogWindow.BPW_DialogWindow_C"))
    (UserInterface|Viewport|AddtoViewport _returnvalue 0)))

(event Input|KeyboardEvents|L
  (params (Key :type Key%20Structure :default "None"))
  (:Pressed
    (bind _returnvalue (UserInterface|CreateWidget "/Game/Blueprints/Widgets/BPW_Leaderboard.BPW_Leaderboard_C"))
    (UserInterface|Viewport|AddtoViewport _returnvalue 0)))

(fn ConstructionScript)